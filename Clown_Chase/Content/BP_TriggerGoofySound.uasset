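; BP_TriggerGoofySound is a one-shot trigger volume that relocates a clown and plays a goofy sound when the player walks in.
; When BP_FirstPersonCharacter overlaps the Box, it teleports the Clown to the ClownPatrol location and sets that as its current patrol point.
; It then plays the sound through GoofySoundsEmettor and sets AlreadyTeleported so it never fires again.
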(event `self.Box.OnComponentBeginOverlap`
  (params (OverlappedComponent :type "PrimitiveComponent Object Reference") (OtherActor :type "Actor Object Reference") (OtherComp :type "PrimitiveComponent Object Reference") (OtherBodyIndex :type Integer) (bFromSweep :type Boolean) (SweepResult :type "HitResult Structure (by ref)"))
  (cast `/Game/FirstPerson/Blueprints/BP_FirstPersonCharacter` OtherActor)
  (if (not (`self.AlreadyTeleported`))
    (`self.K2_SetActorLocation` (`self.Clown`) (`self.K2_GetActorLocation` (`self.ClownPatrol`)) false true)
    (set `/Game/Characters/Clown/Clown.CurrentPatrolPoint` (`self.ClownPatrol`) (`self.Clown`))
    (`/Game/Sounds/BP_GoofySoundsEmettor.PlayGoofySound` (`self.GoofySoundsEmettor`))
    (set `self.AlreadyTeleported` true)))

(fn `UserConstructionScript`)
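; Sound emitter actor that plays goofy sounds at its location at random intervals.
; After an initial delay from BeginPlay, Tick uses a CanPlay flag to play the SC_Goofy sound with attenuation, then waits a random time between MinDelay and MaxDelay before re-arming.
; The first play also triggers a one-off 2D sound, tracked with a play counter.
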(event `self.ReceiveBeginPlay`
  (`KismetSystemLibrary.Delay` 50.0)
  (set `self.CanPlay` true))

(event `self.ReceiveTick`
  (params (DeltaSeconds :type "Float (single-precision)"))
  (if (`self.CanPlay`)
    (set `self.CanPlay` false)
    (`GameplayStatics.PlaySoundAtLocation` "/Game/Sounds/SC_Goofy.SC_Goofy" (`self.K2_GetActorLocation`) (struct) 1.0 1.0 0.0 "/Game/Sounds/DefaultAttenuation.DefaultAttenuation" null null null)
    (bind _output_get (set `self.NbPlayed` (+ (`self.NbPlayed`) 1)))
    (if (== _output_get 1)
      (`GameplayStatics.PlaySound2D` "/Game/Sounds/premier_bruit_goofy_3.premier_bruit_goofy_3" 1.0 1.0 0.0 null null))
    (`KismetSystemLibrary.Delay` (`KismetMathLibrary.RandomFloatInRange` (`self.min_delay`) (`self.max_delay`)))
    (set `self.CanPlay` true)))

(fn `UserConstructionScript`)
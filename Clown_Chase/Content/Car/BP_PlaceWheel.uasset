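; BP_PlaceWheel is an interactable spot in the car folder where the first-person player can place a carried wheel, once.
; A sphere overlap tracks whether the player is in range and caches the character reference.
; Interact asks the character to drop its wheel; on success it plays an inventory sound, reveals the 01CamelSecours component and locks further placement.
; Range changes and failed drops print debug strings.
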(event `self.ReceiveBeginPlay`
  (`self.EnableInput` (`GameplayStatics.GetPlayerController` 0)))

(event `self.Sphere.OnComponentBeginOverlap`
  (params (OverlappedComponent :type "PrimitiveComponent Object Reference") (OtherActor :type "Actor Object Reference") (OtherComp :type "PrimitiveComponent Object Reference") (OtherBodyIndex :type Integer) (bFromSweep :type Boolean) (SweepResult :type "HitResult Structure (by ref)"))
  (bind _asbp_first_person_character (cast `/Game/FirstPerson/Blueprints/BP_FirstPersonCharacter` OtherActor))
  (set `self.InPlayerRange` true)
  (set `self.Player` _asbp_first_person_character)
  (`KismetSystemLibrary.PrintString` "Hello"))

(event `self.Sphere.OnComponentEndOverlap`
  (params (OverlappedComponent :type "PrimitiveComponent Object Reference") (OtherActor :type "Actor Object Reference") (OtherComp :type "PrimitiveComponent Object Reference") (OtherBodyIndex :type Integer))
  (cast `/Game/FirstPerson/Blueprints/BP_FirstPersonCharacter` OtherActor)
  (set `self.InPlayerRange` false)
  (set `self.Player` null)
  (`KismetSystemLibrary.PrintString` "Bye"))

(event `/Game/Car/BPI_Interactable.Interact`
  (if (`self.WheelPlaced`)
    _
    (elif (and (`self.InPlayerRange`) (`KismetSystemLibrary.IsValid` (`self.Player`)))
      (bind _succeed (`/Game/FirstPerson/Blueprints/BP_FirstPersonCharacter.DropWheel` (`self.Player`)))
      (if _succeed
        (`GameplayStatics.PlaySound2D` "/Game/Sounds/inventory.inventory" 1.0 1.0 0.0 null null)
        (`SceneComponent.SetVisibility` (`self.01_camel_secours`) true false)
        (set `self.WheelPlaced` true)
        (else
          (`KismetSystemLibrary.PrintString` "nul"))))))

(fn `UserConstructionScript`)